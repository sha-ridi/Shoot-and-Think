(event `self.ReceiveBeginPlay`
  (`self.Update Targets`))

(event `self.OverlapBox.OnComponentBeginOverlap`
  (params (OverlappedComponent :type "PrimitiveComponent Object Reference") (OtherActor :type "Actor Object Reference") (OtherComp :type "PrimitiveComponent Object Reference") (OtherBodyIndex :type Integer) (bFromSweep :type Boolean) (SweepResult :type "HitResult Structure (by ref)"))
  (if (`self.ActorHasTag` OtherActor "ShootTarget")
    (`self.Update Targets`)))

(event `self.OverlapBox.OnComponentEndOverlap`
  (params (OverlappedComponent :type "PrimitiveComponent Object Reference") (OtherActor :type "Actor Object Reference") (OtherComp :type "PrimitiveComponent Object Reference") (OtherBodyIndex :type Integer))
  (if (`self.ActorHasTag` OtherActor "ShootTarget")
    (`self.Update Targets`)))

(event `Level Cleared`
  (bind (_direction _alpha) (`Timeline|Timeline`)
    (:`Update`
      (`SceneComponent.SetWorldScale3D` (`self.TextRender`) (`KismetMathLibrary.Conv_DoubleToVector` (`KismetMathLibrary.Lerp` 1.0 3.0 _alpha))))
    (:`Finished`
      (if (`self.Is Level Cleared`)
        (set `self.bGoalAchieved` true)
        (if (`self.bFinalLevel`)
          (`TextRenderComponent.K2_SetText` (`self.TextRender`) "You Win")
          (else
            (`SceneComponent.SetVisibility` (`self.TextRender`) false false)
            (`|SpawnActorFromClass` "/Game/Blueprints/BP_NextLevel.BP_NextLevel_C" (`KismetMathLibrary.MakeTransform` (`SceneComponent.K2_GetComponentLocation` (`self.TextRender`))) "Undefined" "MultiplyWithRoot" null null)))
        (else
          (bind _returnvalue (`GameplayStatics.GetCurrentLevelName` true))
          (`GameplayStatics.OpenLevel` (`KismetStringLibrary.Conv_StringToName` _returnvalue)))))))

(fn `Is Level Cleared`
  (returns (ReturnValue :type Boolean))
  (return (== (`self.Targets Count`) (`self.GoalNoumber`))))

(fn `Update Targets`
  (locals (Color :type "Color Structure" :default (struct :`B` 169 :`G` 101 :`R` 88 :`A` 255)))
  (if (not (`self.bGoalAchieved`))
    (bind _output_get (set `self.Overlapping Targets` (`PrimitiveComponent.GetOverlappingActors` (`self.OverlapBox`) "/Game/Blueprints/BP_ShootTarget.BP_ShootTarget_C")))
    (set `self.Targets Count` (`KismetArrayLibrary.Array_Length` _output_get))
    (`TextRenderComponent.K2_SetText` (`self.TextRender`) (`KismetTextLibrary.Conv_IntToText` (`self.Targets Count`)))
    (`TextRenderComponent.K2_SetText` (`self.Goal`) (`KismetTextLibrary.Conv_IntToText` (`self.GoalNoumber`)))
    (if (`self.Is Level Cleared`)
      (`self.Level Cleared`))))

(fn `UserConstructionScript`
  (`PrimitiveComponent.SetMaterial` (`self.Cube`) 0 (`/Game/Blueprints/Game/BFL_Main.Get Random Color Material`)))