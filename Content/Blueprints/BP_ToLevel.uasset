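; BP_ToLevel is a level-transition trigger that shows its LevelName on a Text component at BeginPlay.
; When an actor tagged NextLevelActivate overlaps its Cylinder, a DoOnce gate lets it play an open sound and immediately load that level by name.
; An unconnected Timeline that would shrink the actor's root to zero before opening the level never runs.
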(event `self.ReceiveBeginPlay`
  (`TextRenderComponent.K2_SetText` (`self.Text`) (`KismetTextLibrary.Conv_NameToText` (`self.Level Name`))))

(event `self.Cylinder.OnComponentBeginOverlap`
  (params (OverlappedComponent :type "PrimitiveComponent Object Reference") (OtherActor :type "Actor Object Reference") (OtherComp :type "PrimitiveComponent Object Reference") (OtherBodyIndex :type Integer) (bFromSweep :type Boolean) (SweepResult :type "HitResult Structure (by ref)"))
  (if (`self.ActorHasTag` OtherActor "NextLevelActivate")
    (`/Engine/EditorBlueprintResources/StandardMacros.DoOnce` false
      (:`Completed`
        (`GameplayStatics.PlaySoundAtLocation` "/Game/Packs/UE_Sounds/VR_open_Cue.VR_open_Cue" (`self.K2_GetActorLocation`) (struct) 1.0 1.0 0.0 null null null null)
        (`GameplayStatics.OpenLevel` (`self.Level Name`))))))

(fn `UserConstructionScript`)