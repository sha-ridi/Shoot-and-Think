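; BP_Weapon is a weapon Blueprint that tracks whether the weapon is disabled through a count of deactivators.
; AddDeactivator increments DeactiveCount and calls SetCondition to disable the weapon if it is not already disabled.
; RemoveDeactivator decrements the count and re-enables it only at zero, so overlapping deactivators stack.
; SetCondition is empty here, and nothing in these graphs writes the Disabled flag.
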(event `SetCondition`
  (params (Disabled :type Boolean)))

(fn `Add Deactivator`
  (`/Engine/EditorBlueprintResources/StandardMacros.IncrementInt` (`self.DeactiveCount`)
    (:`  `
      (if (not (`self.bDisabled`))
        (`self.SetCondition` true)))))

(fn `Remove Deactivator`
  (bind _result (`/Engine/EditorBlueprintResources/StandardMacros.DecrementInt` (`self.DeactiveCount`))
    (:`  `
      (if (== _result 0)
        (if (`self.bDisabled`)
          (`self.SetCondition` false))))))

(fn `UserConstructionScript`)