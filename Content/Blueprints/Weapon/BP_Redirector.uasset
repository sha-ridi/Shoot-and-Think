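; BP_Redirector is a weapon-related actor that responds to an overlapping projectile by firing a new BP_Projectile from its own spawn point and direction.
; Overlaps with "Projectile"-tagged actors spawn the new projectile at the incoming one's scale, throttled by a short time check and switchable through SetCondition.
; The mesh gets a random material at construction and BeginPlay.
; A looping auto-fire timer is left unconnected.
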(event `self.ReceiveBeginPlay`
  (`PrimitiveComponent.SetMaterial` (`self.StaticMesh`) 0 (`/Game/Blueprints/Game/BFL_Main.Get Random Material` false)))

(event `CustomEvent`
  (bind _projectilespawn (`self.ProjectileSpawn`))
  (`|SpawnActorFromClass` "/Game/Blueprints/Weapon/BP_Projectile.BP_Projectile_C" (`KismetMathLibrary.MakeTransform` (`SceneComponent.K2_GetComponentLocation` _projectilespawn) (`SceneComponent.K2_GetComponentRotation` _projectilespawn)) "Undefined" "OverrideRootScale" null null))

(event `self.ReceiveActorBeginOverlap`
  (params (OtherActor :type "Actor Object Reference"))
  (bind _projectilespawn (`self.ProjectileSpawn`))
  (if (not (`self.bDisabled`))
    (bind _output_get (set `self.CurrentTime` (`KismetSystemLibrary.GetGameTimeInSeconds`)))
    (if (>= (- _output_get (`self.LastCallTime`)) 0.09)
      (set `self.LastCallTime` (`self.CurrentTime`))
      (if (`self.ActorHasTag` OtherActor "Projectile")
        (`|SpawnActorFromClass` "/Game/Blueprints/Weapon/BP_Projectile.BP_Projectile_C" (`KismetMathLibrary.MakeTransform` (`SceneComponent.K2_GetComponentLocation` _projectilespawn) (`SceneComponent.K2_GetComponentRotation` _projectilespawn) (`self.GetActorScale3D` OtherActor)) "Undefined" "OverrideRootScale" null null)))))

(event `self.SetCondition`
  (params (Disabled :type Boolean))
  (set `self.bDisabled` Disabled))

(fn `UserConstructionScript`
  (`PrimitiveComponent.SetMaterial` (`self.StaticMesh`) 0 (`/Game/Blueprints/Game/BFL_Main.Get Random Material` false))
  (`ArrowComponent.SetArrowColor` (`self.Arrow`) (struct :`R` 2.141904 :`G` 2.849955 :`B` 3.0 :`A` 1.0)))