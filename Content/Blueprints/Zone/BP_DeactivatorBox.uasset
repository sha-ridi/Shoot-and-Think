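; BP_DeactivatorBox is a zone actor that disables any BP_Weapon inside its box while keeping it visible to the player.
; On BeginPlay it disables weapons already overlapping, then disables on begin overlap and re-enables on end overlap through SetCondition.
; The construction script scales the point light's attenuation radius and the NSDeactivation effect's BoxSize parameter from the box's world scale, so visuals match the volume.
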(event `self.ReceiveBeginPlay`
  (for _array_element (`PrimitiveComponent.GetOverlappingActors` (`self.Box`) "/Game/Blueprints/Weapon/BP_Weapon.BP_Weapon_C")
    (bind _asbp_weapon (cast `/Game/Blueprints/Weapon/BP_Weapon` _array_element))
    (`/Game/Blueprints/Weapon/BP_Riffle.SetCondition` _asbp_weapon true false)))

(event `self.Box.OnComponentBeginOverlap`
  (params (OverlappedComponent :type "PrimitiveComponent Object Reference") (OtherActor :type "Actor Object Reference") (OtherComp :type "PrimitiveComponent Object Reference") (OtherBodyIndex :type Integer) (bFromSweep :type Boolean) (SweepResult :type "HitResult Structure (by ref)"))
  (bind _asbp_weapon (cast `/Game/Blueprints/Weapon/BP_Weapon` OtherActor))
  (`/Game/Blueprints/Weapon/BP_Riffle.SetCondition` _asbp_weapon true false))

(event `self.Box.OnComponentEndOverlap`
  (params (OverlappedComponent :type "PrimitiveComponent Object Reference") (OtherActor :type "Actor Object Reference") (OtherComp :type "PrimitiveComponent Object Reference") (OtherBodyIndex :type Integer))
  (bind _asbp_weapon (cast `/Game/Blueprints/Weapon/BP_Weapon` OtherActor))
  (`/Game/Blueprints/Weapon/BP_Riffle.SetCondition` _asbp_weapon false false))

(fn `UserConstructionScript`
  (bind _returnvalue (`SceneComponent.K2_GetComponentScale` (`self.Box`)))
  (`LocalLightComponent.SetAttenuationRadius` (`self.PointLight`) (* (.x _returnvalue) 120.0))
  (`FXSystemComponent.SetVectorParameter` (`self.NS_Deactivation`) "BoxSize" (* _returnvalue 100.0)))