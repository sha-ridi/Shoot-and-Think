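; BP_Target is a level objective that activates when a BP_Projectile with a matching Twin flag overlaps its main cylinder.
; On BeginPlay it registers as an activatable with BP_LevelController and applies its optional physics setting.
; The first valid hit turns it green, plays a sound and asks the controller to end the level if it was last.
; SetColor swaps materials on four cylinders, with the inactive look depending on Twin, and also runs at construction.
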(event `self.ReceiveBeginPlay`
  (`self.SetColor` false)
  (bind _returnvalue (`GameplayStatics.GetActorOfClass` "/Game/Blueprints/Level/BP_LevelController.BP_LevelController_C"))
  (bind _output_get (set `self.Level Controller` _returnvalue))
  (`/Game/Blueprints/Level/BP_LevelController.Add Activatable` _output_get)
  (`PrimitiveComponent.SetSimulatePhysics` (`self.Cylinder`) (`self.bSimulatePhysics`)))

(event `self.Cylinder.OnComponentBeginOverlap`
  (params (OverlappedComponent :type "PrimitiveComponent Object Reference") (OtherActor :type "Actor Object Reference") (OtherComp :type "PrimitiveComponent Object Reference") (OtherBodyIndex :type Integer) (bFromSweep :type Boolean) (SweepResult :type "HitResult Structure (by ref)"))
  (bind _asbp_projectile (cast `/Game/Blueprints/Weapon/BP_Projectile` OtherActor))
  (if (== (`/Game/Blueprints/Weapon/BP_Projectile.bTwin` _asbp_projectile) (`self.bTwin`))
    (`/Engine/EditorBlueprintResources/StandardMacros.DoOnce` false
      (:`Completed`
        (`self.SetColor` true)
        (`/Game/Blueprints/Level/BP_LevelController.End Level if Last` (`self.Level Controller`))
        (`GameplayStatics.PlaySoundAtLocation` "/Game/Assets/Audio/Book_Handle_1-5_Cue.Book_Handle_1-5_Cue" (`self.K2_GetActorLocation`) (struct) 1.0 1.0 0.0 null null null null)))))

(fn `SetColor`
  (params (bGreen :type Boolean))
  (if (`self.bTwin`)
    (`PrimitiveComponent.SetMaterial` (`self.Cylinder`) 0 (select `bool` (`local.bGreen`) :`false` "/Game/Assets/Materials/M_DeactiveFloor.M_DeactiveFloor" :`true` "/Game/Assets/Materials/Colors/MI_Green.MI_Green" :!type "MaterialInterface Object Reference"))
    (`PrimitiveComponent.SetMaterial` (`self.Cylinder2`) 0 (select `bool` (`local.bGreen`) :`false` "/Game/Assets/Materials/M_DeactiveFloor.M_DeactiveFloor" :`true` "/Game/Assets/Materials/Colors/MI_Green.MI_Green" :!type "MaterialInterface Object Reference"))
    (`PrimitiveComponent.SetMaterial` (`self.Cylinder3`) 0 (select `bool` (`local.bGreen`) :`false` "/Game/Assets/Materials/M_VisWall.M_VisWall" :`true` "/Game/Assets/Materials/Emissive/MI_EmissiveGreen.MI_EmissiveGreen" :!type "MaterialInterface Object Reference"))
    (`PrimitiveComponent.SetMaterial` (`self.Cylinder1`) 0 (select `bool` (`local.bGreen`) :`false` "/Game/Assets/Materials/M_VisWall.M_VisWall" :`true` "/Game/Assets/Materials/Emissive/MI_EmissiveGreen.MI_EmissiveGreen" :!type "MaterialInterface Object Reference"))
    (else
      (`PrimitiveComponent.SetMaterial` (`self.Cylinder`) 0 (select `bool` (`local.bGreen`) :`false` "/Game/Assets/Materials/Colors/MI_Red.MI_Red" :`true` "/Game/Assets/Materials/Colors/MI_Green.MI_Green" :!type "MaterialInterface Object Reference"))
      (`PrimitiveComponent.SetMaterial` (`self.Cylinder2`) 0 (select `bool` (`local.bGreen`) :`false` "/Game/Assets/Materials/Colors/MI_Red.MI_Red" :`true` "/Game/Assets/Materials/Colors/MI_Green.MI_Green" :!type "MaterialInterface Object Reference"))
      (`PrimitiveComponent.SetMaterial` (`self.Cylinder3`) 0 (select `bool` (`local.bGreen`) :`false` "/Game/Assets/Materials/Emissive/MI_EmissiveRed.MI_EmissiveRed" :`true` "/Game/Assets/Materials/Emissive/MI_EmissiveGreen.MI_EmissiveGreen" :!type "MaterialInterface Object Reference"))
      (`PrimitiveComponent.SetMaterial` (`self.Cylinder1`) 0 (select `bool` (`local.bGreen`) :`false` "/Game/Assets/Materials/Emissive/MI_EmissiveRed.MI_EmissiveRed" :`true` "/Game/Assets/Materials/Emissive/MI_EmissiveGreen.MI_EmissiveGreen" :!type "MaterialInterface Object Reference")))))

(fn `UserConstructionScript`
  (`self.SetColor` false))