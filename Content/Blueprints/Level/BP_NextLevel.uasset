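; BP_NextLevel is a level exit that loads the next level when a tagged actor touches it.
; On BeginPlay it plays a start sound and grows from zero scale via a timeline, arming itself once finished.
; An overlap on its Cylinder by an actor tagged NextLevelActivate then triggers, once only, an end sound and a shrink timeline.
; When the shrink finishes, it opens the level returned by GetNextLevelName.
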(event `self.ReceiveBeginPlay`
  (`GameplayStatics.PlaySoundAtLocation` "/Game/Packs/UE_Sounds/StartSimulate_Cue.StartSimulate_Cue" (`self.K2_GetActorLocation`) (struct) 1.0 1.0 0.0 null null null null)
  (bind (_direction _alpha) (`Timeline|Timeline_0`)
    (:`Update`
      (`SceneComponent.SetWorldScale3D` (`self.DefaultSceneRoot`) (`KismetMathLibrary.VLerp` (0.0 0.0 0.0) (2.0 2.0 2.0) _alpha)))
    (:`Finished`
      (set `self.bSpawned` true))))

(event `self.Cylinder.OnComponentBeginOverlap`
  (params (OverlappedComponent :type "PrimitiveComponent Object Reference") (OtherActor :type "Actor Object Reference") (OtherComp :type "PrimitiveComponent Object Reference") (OtherBodyIndex :type Integer) (bFromSweep :type Boolean) (SweepResult :type "HitResult Structure (by ref)"))
  (if (`self.bSpawned`)
    (if (`self.ActorHasTag` OtherActor "NextLevelActivate")
      (`/Engine/EditorBlueprintResources/StandardMacros.DoOnce` false
        (:`Completed`
          (`GameplayStatics.PlaySoundAtLocation` "/Game/Packs/UE_Sounds/EndSimulate_Cue.EndSimulate_Cue" (`self.K2_GetActorLocation`) (struct) 1.0 1.0 0.0 null null null null)
          (bind (_direction _alpha) (`Timeline|Timeline`)
            (:`Update`
              (`SceneComponent.SetWorldScale3D` (`self.DefaultSceneRoot`) (`KismetMathLibrary.VLerp` (2.0 2.0 2.0) (0.0 0.0 0.0) _alpha)))
            (:`Finished`
              (`GameplayStatics.OpenLevel` (`/Game/Blueprints/Game/BFL_Main.Get Next Level Name`)))))))))

(fn `UserConstructionScript`)