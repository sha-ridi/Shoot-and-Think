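; BP_LevelController tracks a level's completion and spawns the follow-on actor once every activatable is done.
; AddActivatable increments a counter, and EndLevelIfLast decrements it, calling CompleteLevel when it reaches zero.
; CompleteLevel spawns BP_NextLevel at the controller's own location, or BP_ToLobby when FinalLevel is set.
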(event `Complete Level`
  (`|SpawnActorFromClass` (select `bool` (`self.bFinalLevel`) :`false` "/Game/Blueprints/Level/BP_NextLevel.BP_NextLevel_C" :`true` "/Game/Blueprints/Level/BP_ToLobby.BP_ToLobby_C" :!type "Actor Class Reference") (`KismetMathLibrary.MakeTransform` (`self.K2_GetActorLocation`)) "Undefined" "MultiplyWithRoot" null null))

(fn `Add Activatable`
  (`/Engine/EditorBlueprintResources/StandardMacros.IncrementInt` (`self.ActivatableCount`)))

(fn `End Level if Last`
  (`/Engine/EditorBlueprintResources/StandardMacros.DecrementInt` (`self.ActivatableCount`)
    (:`  `
      (if (`self.Is All Activated`)
        (`self.Complete Level`)))))

(fn `Is All Activated`
  (returns (ReturnValue :type Boolean))
  (return (== (`self.ActivatableCount`) 0)))

(fn `UserConstructionScript`)