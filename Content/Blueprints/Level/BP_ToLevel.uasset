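; A grabbable level-select object that displays its level number and loads that level when picked up.
; Three text components show the Level number, tinted with the Color variable in the construction script.
; UpdateAppearance swaps the mesh between emissive and plain blue materials and toggles its collision to match availability.
; Grabbing it through BP_GrabComponent plays a timeline that shrinks the mesh to nothing, then opens the level resolved from the integer.
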(event `Update Appearance`
  (params (bAvailable :type Boolean))
  (set `self.bAvailiable` bAvailable)
  (`PrimitiveComponent.SetMaterial` (`self.Mesh`) 0 (select `bool` (`self.bAvailiable`) :`false` "/Game/Assets/Materials/MI_Blue0.MI_Blue0" :`true` "/Game/Assets/Riffle/MI_BlueEmissive.MI_BlueEmissive" :!type "MaterialInterface Object Reference"))
  (`PrimitiveComponent.SetCollisionEnabled` (`self.Mesh`) (select `bool` (`self.bAvailiable`) :`false` "NoCollision" :`true` "QueryAndPhysics" :!type "ECollisionEnabled Enum")))

(event `self.ReceiveBeginPlay`
  (`TextRenderComponent.K2_SetText` (`self.Text`) (`KismetTextLibrary.Conv_IntToText` (`self.Level`)))
  (`TextRenderComponent.K2_SetText` (`self.Text1`) (`KismetTextLibrary.Conv_IntToText` (`self.Level`)))
  (`TextRenderComponent.K2_SetText` (`self.Text2`) (`KismetTextLibrary.Conv_IntToText` (`self.Level`))))

(event `self.BP_GrabComponent.OnGrabbed`
  (bind (_direction _alpha) (`Timeline|Timeline`)
    (:`Update`
      (`SceneComponent.SetWorldScale3D` (`self.Mesh`) (`KismetMathLibrary.VLerp` (`KismetMathLibrary.Conv_DoubleToVector` 0.2) (0.0 0.0 0.0) _alpha)))
    (:`Finished`
      (`GameplayStatics.OpenLevel` (`/Game/Blueprints/Game/BFL_Main.Get Level Name From Integer` (`self.Level`))))))

(fn `UserConstructionScript`
  (locals (Color :type "Color Structure" :default (struct :`B` 255 :`G` 135 :`A` 255)))
  (`TextRenderComponent.SetTextRenderColor` (`self.Text`) (`local.Color`))
  (`TextRenderComponent.SetTextRenderColor` (`self.Text1`) (`local.Color`))
  (`TextRenderComponent.SetTextRenderColor` (`self.Text2`) (`local.Color`)))