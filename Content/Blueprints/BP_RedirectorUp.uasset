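; Redirector actor that catches tagged projectiles on an elevated mesh and spawns a new one along its ProjectileSpawn direction, raised by Height.
; Overlaps are time-throttled, and the new projectile copies the incoming scale and uses the actor's Speed.
; Construction sizes the meshes from Height, while Tick keeps the upper mesh above the optionally physics-simulated base.
; A predicted trajectory feeds a Niagara path and impact sphere; Test mode fires projectiles on a timer.
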(event `self.ReceiveBeginPlay`
  (`PrimitiveComponent.SetSimulatePhysics` (`self.StaticMesh`) (`self.bSimulatePhysics`))
  (`PrimitiveComponent.SetEnableGravity` (`self.StaticMesh`) (`self.bGravity`))
  (`PrimitiveComponent.SetMaterial` (`self.StaticMesh`) 0 (`/Game/Blueprints/Game/BFL_Main.Get Random Material` false))
  (if (`self.bTest`)
    (`KismetSystemLibrary.K2_SetTimerDelegate` (delegate `CustomEvent`) 0.1 true)))

(event `CustomEvent`
  (bind _projectilespawn (`self.ProjectileSpawn`))
  (`|SpawnActorFromClass` "/Game/Blueprints/Weapon/BP_Projectile.BP_Projectile_C" (`KismetMathLibrary.MakeTransform` (`SceneComponent.K2_GetComponentLocation` _projectilespawn) (`SceneComponent.K2_GetComponentRotation` _projectilespawn)) "Undefined" "OverrideRootScale" null (`self.Speed`) null))

(event `self.StaticMesh1.OnComponentBeginOverlap`
  (params (OverlappedComponent :type "PrimitiveComponent Object Reference") (OtherActor :type "Actor Object Reference") (OtherComp :type "PrimitiveComponent Object Reference") (OtherBodyIndex :type Integer) (bFromSweep :type Boolean) (SweepResult :type "HitResult Structure (by ref)"))
  (bind _projectilespawn (`self.ProjectileSpawn`))
  (bind _output_get (set `self.CurrentTime` (`KismetSystemLibrary.GetGameTimeInSeconds`)))
  (if (>= (- _output_get (`self.LastCallTime`)) 0.09)
    (set `self.LastCallTime` (`self.CurrentTime`))
    (if (`self.ActorHasTag` OtherActor "Projectile")
      (`|SpawnActorFromClass` "/Game/Blueprints/Weapon/BP_Projectile.BP_Projectile_C" (`KismetMathLibrary.MakeTransform` (+ (`SceneComponent.K2_GetComponentLocation` _projectilespawn) (`KismetMathLibrary.MakeVector` 0.0 0.0 (`self.Height`))) (`SceneComponent.K2_GetComponentRotation` _projectilespawn) (`self.GetActorScale3D` OtherActor)) "Undefined" "OverrideRootScale" null (`self.Speed`) null))))

(event `self.ReceiveTick`
  (params (DeltaSeconds :type "Float (single-precision)"))
  (bind (_returnvalue_location _returnvalue_rotation _returnvalue_scale) (`KismetMathLibrary.BreakTransform` (`SceneComponent.K2_GetComponentToWorld` (`self.StaticMesh`))))
  (`self.Draw Trace`)
  (`SceneComponent.K2_SetWorldTransform` (`self.StaticMesh1`) (`KismetMathLibrary.MakeTransform` (+ _returnvalue_location (`KismetMathLibrary.MakeVector` 0.0 0.0 (`self.Height`))) _returnvalue_rotation _returnvalue_scale) false false))

(fn `Draw Trace`
  (bind _projectilespawn (`self.ProjectileSpawn`))
  (`|ExecutionSequence`
    (:`then_0`
      (bind (_outhit _outpathpositions _outlasttracedestination _returnvalue) (`GameplayStatics.Blueprint_PredictProjectilePath_ByTraceChannel` (+ (`SceneComponent.K2_GetComponentLocation` _projectilespawn) (`KismetMathLibrary.MakeVector` 0.0 0.0 (`self.Height`))) (* (`SceneComponent.GetForwardVector` _projectilespawn) (`self.Speed`)) true 10.0 "ECC_Visibility" false (`|MakeArray` self :!type "Actor Object Reference") "None" 0.0 15.0 5.0))
      (bind _output_get (set `self.Out Path Positions` _outpathpositions))
      (`KismetArrayLibrary.Array_Insert` _output_get (+ (`self.K2_GetActorLocation`) (`KismetMathLibrary.MakeVector` 0.0 0.0 (`self.Height`))))
      (if _returnvalue
        (`SceneComponent.K2_SetWorldLocation` (`self.Sphere`) (`.Location` (`GameplayStatics.BreakHitResult` _outhit)) false false)
        (else
          (`SceneComponent.K2_SetRelativeLocation` (`self.Sphere`) (0.0 0.0 0.0) false false))))
    (:`then_1`
      (`NiagaraDataInterfaceArrayFunctionLibrary.SetNiagaraArrayVector` (`self.Niagara`) "User.PointArray" (`self.Out Path Positions`)))))

(fn `UserConstructionScript`
  (`PrimitiveComponent.SetMaterial` (`self.StaticMesh`) 0 (`/Game/Blueprints/Game/BFL_Main.Get Random Material` false))
  (`PrimitiveComponent.SetMaterial` (`self.StaticMesh1`) 0 (`/Game/Blueprints/Game/BFL_Main.Get Random Material` false))
  (`PrimitiveComponent.SetMaterial` (`self.StaticMesh2`) 0 (`/Game/Blueprints/Game/BFL_Main.Get Random Material` false))
  (`SceneComponent.K2_SetRelativeLocation` (`self.StaticMesh1`) (`KismetMathLibrary.MakeVector` 0.0 0.0 (* (`self.Height`) 5.0)) false false)
  (`SceneComponent.SetRelativeScale3D` (`self.StaticMesh2`) (`KismetMathLibrary.MakeVector` 0.3 0.3 (* (`self.Height`) 0.05)))
  (`self.Draw Trace`))