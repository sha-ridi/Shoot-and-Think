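; BP_BubbleCube is a cube Blueprint that gives its mesh a random material and a random uniform scale for visual variety.
; The construction script applies both through GetRandomMaterial and a bounded random float.
; BeginPlay repeats the same randomization, so the look rolled at construction is replaced when play starts.
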(event `self.ReceiveBeginPlay`
  (`PrimitiveComponent.SetMaterial` (`self.Mesh`) 0 (`/Game/Blueprints/Game/BFL_Main.Get Random Material` true))
  (`SceneComponent.SetWorldScale3D` (`self.Mesh`) (`KismetMathLibrary.Conv_DoubleToVector` (`KismetMathLibrary.RandomFloatInRange` 0.2 0.6))))

(fn `UserConstructionScript`
  (`SceneComponent.SetWorldScale3D` (`self.Mesh`) (`KismetMathLibrary.Conv_DoubleToVector` (`KismetMathLibrary.RandomFloatInRange` 0.2 0.6)))
  (`PrimitiveComponent.SetMaterial` (`self.Mesh`) 0 (`/Game/Blueprints/Game/BFL_Main.Get Random Material` true)))