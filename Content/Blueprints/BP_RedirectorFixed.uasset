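; Fixed redirector actor that, when overlapped by a Projectile-tagged actor, spawns a new BP_Projectile from its spawn point at the incoming actor's scale.
; A short time gate throttles overlap handling.
; Tick and the construction script predict the outgoing arc and feed its points to a Niagara array for a trajectory preview.
; Mesh material is randomized; a timed test-firing branch is left unconnected.
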(event `self.ReceiveBeginPlay`
  (`PrimitiveComponent.SetMaterial` (`self.StaticMesh`) 0 (`/Game/Blueprints/Game/BFL_Main.Get Random Material` false)))

(event `CustomEvent`
  (bind _projectilespawn (`self.ProjectileSpawn`))
  (`|SpawnActorFromClass` "/Game/Blueprints/Weapon/BP_Projectile.BP_Projectile_C" (`KismetMathLibrary.MakeTransform` (`SceneComponent.K2_GetComponentLocation` _projectilespawn) (`SceneComponent.K2_GetComponentRotation` _projectilespawn)) "Undefined" "OverrideRootScale" null null))

(event `self.ReceiveActorBeginOverlap`
  (params (OtherActor :type "Actor Object Reference"))
  (bind _projectilespawn (`self.ProjectileSpawn`))
  (bind _output_get (set `self.CurrentTime` (`KismetSystemLibrary.GetGameTimeInSeconds`)))
  (if (>= (- _output_get (`self.LastCallTime`)) 0.09)
    (set `self.LastCallTime` (`self.CurrentTime`))
    (if (`self.ActorHasTag` OtherActor "Projectile")
      (`|SpawnActorFromClass` "/Game/Blueprints/Weapon/BP_Projectile.BP_Projectile_C" (`KismetMathLibrary.MakeTransform` (`SceneComponent.K2_GetComponentLocation` _projectilespawn) (`SceneComponent.K2_GetComponentRotation` _projectilespawn) (`self.GetActorScale3D` OtherActor)) "Undefined" "OverrideRootScale" null null))))

(event `self.ReceiveTick`
  (params (DeltaSeconds :type "Float (single-precision)"))
  (bind _projectilespawn (`self.ProjectileSpawn`))
  (`|ExecutionSequence`
    (:`then_0`
      (bind (_outhit _outpathpositions) (`GameplayStatics.Blueprint_PredictProjectilePath_ByTraceChannel` (`SceneComponent.K2_GetComponentLocation` _projectilespawn) (* (`SceneComponent.GetForwardVector` _projectilespawn) 1000.0) true 10.0 "ECC_Visibility"))
      (set `self.Out Path Positions` _outpathpositions))
    (:`then_1`
      (`NiagaraDataInterfaceArrayFunctionLibrary.SetNiagaraArrayVector` (`self.Niagara`) "User.PointArray" (`self.Out Path Positions`)))))

(fn `UserConstructionScript`
  (bind _projectilespawn (`self.ProjectileSpawn`))
  (`PrimitiveComponent.SetMaterial` (`self.StaticMesh`) 0 (`/Game/Blueprints/Game/BFL_Main.Get Random Material` false))
  (`|ExecutionSequence`
    (:`then_0`
      (bind (_outhit _outpathpositions) (`GameplayStatics.Blueprint_PredictProjectilePath_ByTraceChannel` (`SceneComponent.K2_GetComponentLocation` _projectilespawn) (* (`SceneComponent.GetForwardVector` _projectilespawn) 1000.0) true 10.0 "ECC_Visibility"))
      (set `self.Out Path Positions` _outpathpositions))
    (:`then_1`
      (`NiagaraDataInterfaceArrayFunctionLibrary.SetNiagaraArrayVector` (`self.Niagara`) "User.PointArray" (`self.Out Path Positions`)))))