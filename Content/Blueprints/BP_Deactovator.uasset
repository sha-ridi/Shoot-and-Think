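; BP_Deactovator is a zone actor that toggles the condition on any BP_Riffle entering it, apparently as a deactivator.
; Sphere overlap begin sets the rifle's condition to true, and overlap end sets it back to false.
; The construction script derives the PointLight's attenuation radius from the sphere's world Z scale, so the light scales with the zone.
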(event `self.Sphere.OnComponentBeginOverlap`
  (params (OverlappedComponent :type "PrimitiveComponent Object Reference") (OtherActor :type "Actor Object Reference") (OtherComp :type "PrimitiveComponent Object Reference") (OtherBodyIndex :type Integer) (bFromSweep :type Boolean) (SweepResult :type "HitResult Structure (by ref)"))
  (bind _asbp_riffle (cast `/Game/Blueprints/Weapon/BP_Riffle` OtherActor))
  (`/Game/Blueprints/Weapon/BP_Riffle.SetCondition` _asbp_riffle true))

(event `self.Sphere.OnComponentEndOverlap`
  (params (OverlappedComponent :type "PrimitiveComponent Object Reference") (OtherActor :type "Actor Object Reference") (OtherComp :type "PrimitiveComponent Object Reference") (OtherBodyIndex :type Integer))
  (bind _asbp_riffle (cast `/Game/Blueprints/Weapon/BP_Riffle` OtherActor))
  (`/Game/Blueprints/Weapon/BP_Riffle.SetCondition` _asbp_riffle false))

(fn `UserConstructionScript`
  (bind (_returnvalue_x _returnvalue_y _returnvalue_z) (`KismetMathLibrary.BreakVector` (`SceneComponent.K2_GetComponentScale` (`self.Sphere`))))
  (`LocalLightComponent.SetAttenuationRadius` (`self.PointLight`) (* _returnvalue_z 100.0)))