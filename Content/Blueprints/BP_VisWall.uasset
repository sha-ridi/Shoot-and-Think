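; BP_VisWall is an actor built from four bar cubes and four small cubes, with all logic in its construction script.
; The script pins the bars to a thin cross-section, keeping the Y scale of one pair and the X scale of the other.
; It then applies a material from GetRandomMaterial to all eight cubes.
; The event graph holds only disabled placeholder events.
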(fn `UserConstructionScript`
  (bind _returnvalue_x (`KismetMathLibrary.BreakVector` (`SceneComponent.K2_GetComponentScale` (`self.Cube2`))))
  (bind (_returnvalue_x_2 _returnvalue_y) (`KismetMathLibrary.BreakVector` (`SceneComponent.K2_GetComponentScale` (`self.Cube`))))
  (`SceneComponent.SetWorldScale3D` (`self.Cube`) (`KismetMathLibrary.MakeVector` 0.1 _returnvalue_y 0.1))
  (`SceneComponent.SetWorldScale3D` (`self.Cube1`) (`KismetMathLibrary.MakeVector` 0.1 _returnvalue_y 0.1))
  (`SceneComponent.SetWorldScale3D` (`self.Cube2`) (`KismetMathLibrary.MakeVector` _returnvalue_x 0.1 0.1))
  (`SceneComponent.SetWorldScale3D` (`self.Cube3`) (`KismetMathLibrary.MakeVector` _returnvalue_x 0.1 0.1))
  (`PrimitiveComponent.SetMaterial` (`self.Cube1`) 0 (`/Game/Blueprints/Game/BFL_Main.Get Random Material`))
  (`PrimitiveComponent.SetMaterial` (`self.Cube`) 0 (`/Game/Blueprints/Game/BFL_Main.Get Random Material`))
  (`PrimitiveComponent.SetMaterial` (`self.Cube2`) 0 (`/Game/Blueprints/Game/BFL_Main.Get Random Material`))
  (`PrimitiveComponent.SetMaterial` (`self.Cube3`) 0 (`/Game/Blueprints/Game/BFL_Main.Get Random Material`))
  (`PrimitiveComponent.SetMaterial` (`self.SmallCube`) 0 (`/Game/Blueprints/Game/BFL_Main.Get Random Material`))
  (`PrimitiveComponent.SetMaterial` (`self.SmallCube1`) 0 (`/Game/Blueprints/Game/BFL_Main.Get Random Material`))
  (`PrimitiveComponent.SetMaterial` (`self.SmallCube2`) 0 (`/Game/Blueprints/Game/BFL_Main.Get Random Material`))
  (`PrimitiveComponent.SetMaterial` (`self.SmallCube3`) 0 (`/Game/Blueprints/Game/BFL_Main.Get Random Material`)))