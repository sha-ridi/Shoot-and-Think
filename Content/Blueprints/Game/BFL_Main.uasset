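; Blueprint function library with shared helpers for random blue-themed visuals and numbered level naming.
; Material picks return a main and a twin blue material, with a flag switching the main one to bubble variants.
; Color helpers randomly choose from four blue-toned palettes entries, either standard or over-bright emissive.
; Level helpers rely on the "Level" plus number naming convention to parse the current index and build next or arbitrary level names.
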(fn `Get Current Level`
  (returns (ReturnValue :type Integer))
  (bind _returnvalue (`GameplayStatics.GetCurrentLevelName` null))
  (return (`KismetStringLibrary.Conv_StringToInt` (`KismetStringLibrary.Replace` _returnvalue "Level"))))

(fn `Get Level Name From Integer`
  (params (InInt :type Integer))
  (returns (ReturnValue :type Name))
  (return (`KismetStringLibrary.Conv_StringToName` (`KismetStringLibrary.Concat_StrStr` "Level" (`KismetStringLibrary.Conv_IntToString` InInt)))))

(fn `Get Next Level Name`
  (returns (ReturnValue :type Name))
  (bind _returnvalue (`GameplayStatics.GetCurrentLevelName` null))
  (bind _result (`/Engine/EditorBlueprintResources/StandardMacros.IncrementInt` (`KismetStringLibrary.Conv_StringToInt` (`KismetStringLibrary.Replace` _returnvalue "Level")))
    (:`  `
      (return (`KismetStringLibrary.Conv_StringToName` (`KismetStringLibrary.Concat_StrStr` "Level" (`KismetStringLibrary.Conv_IntToString` _result)))))))

(fn `Get Random Emissive Linear Color`
  (returns (`Return Value` :type "LinearColor Structure"))
  (return (select `int` (`KismetMathLibrary.RandomIntegerInRange` 0 3) :`0` (struct :`R` 1.134324 :`G` 1.576378 :`B` 3.0 :`A` 1.0) :`1` (struct :`R` 0.138379 :`G` 1.591062 :`B` 3.0 :`A` 1.0) :`2` (struct :`R` 1.147533 :`G` 2.118263 :`B` 3.0 :`A` 1.0) :`3` (struct :`R` 2.238332 :`G` 2.760732 :`B` 3.0 :`A` 1.0) :!type "LinearColor Structure")))

(fn `Get Random Linear Color`
  (returns (`Return Value` :type "LinearColor Structure"))
  (return (select `int` (`KismetMathLibrary.RandomIntegerInRange` 0 3) :`0` (struct :`R` 0.006995 :`G` 0.009721 :`B` 0.0185 :`A` 1.0) :`1` (struct :`R` 0.012286 :`G` 0.141263 :`B` 0.266356 :`A` 1.0) :`2` (struct :`R` 0.187821 :`G` 0.346704 :`B` 0.491021 :`A` 1.0) :`3` (struct :`R` 0.539479 :`G` 0.665387 :`B` 0.723055 :`A` 1.0) :!type "LinearColor Structure")))

(fn `Get Random Material`
  (params (bBuble :type Boolean))
  (returns (ReturnValue :type "MaterialInterface Object Reference") (TwinReturnValue :type "MaterialInterface Object Reference"))
  (bind _returnvalue (`KismetMathLibrary.RandomIntegerInRange` 0 3))
  (bind _returnvalue_2 (`KismetMathLibrary.RandomIntegerInRange` 0 3))
  (if bBuble
    (return (select `int` _returnvalue :`0` "/Game/Assets/Materials/Colors/MI_BubbleBlue0.MI_BubbleBlue0" :`1` "/Game/Assets/Materials/Colors/MI_BubbleBlue1.MI_BubbleBlue1" :`2` "/Game/Assets/Materials/Colors/MI_BubbleBlue2.MI_BubbleBlue2" :`3` "/Game/Assets/Materials/Colors/MI_BubbleBlue3.MI_BubbleBlue3" :!type "MaterialInterface Object Reference") (select `int` _returnvalue :`0` "/Game/Assets/Materials/Twin/M_TwinBlue0.M_TwinBlue0" :`1` "/Game/Assets/Materials/Twin/MI_TwinBlue1.MI_TwinBlue1" :`2` "/Game/Assets/Materials/Twin/MI_TwinBlue2.MI_TwinBlue2" :`3` "/Game/Assets/Materials/Twin/MI_TwinBlue3.MI_TwinBlue3" :!type "MaterialInterface Object Reference"))
    (else
      (return (select `int` _returnvalue_2 :`0` "/Game/Assets/Materials/Colors/MI_Blue0.MI_Blue0" :`1` "/Game/Assets/Materials/Colors/MI_Blue1.MI_Blue1" :`2` "/Game/Assets/Materials/Colors/MI_Blue3.MI_Blue3" :`3` "/Game/Assets/Materials/Colors/MI_Blue2.MI_Blue2" :!type "MaterialInterface Object Reference") (select `int` _returnvalue_2 :`0` "/Game/Assets/Materials/Twin/M_TwinBlue0.M_TwinBlue0" :`1` "/Game/Assets/Materials/Twin/MI_TwinBlue1.MI_TwinBlue1" :`2` "/Game/Assets/Materials/Twin/MI_TwinBlue2.MI_TwinBlue2" :`3` "/Game/Assets/Materials/Twin/MI_TwinBlue3.MI_TwinBlue3" :!type "MaterialInterface Object Reference")))))