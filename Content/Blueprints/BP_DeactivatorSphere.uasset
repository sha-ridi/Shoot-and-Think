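; BP_DeactivatorSphere is an area that disables weapons inside it.
; When a BP_Weapon begins overlapping its Sphere, it calls SetCondition to disable it while keeping it visible to the player, and re-enables it on end overlap.
; The construction script derives a radius from the Sphere's world Z scale to size the point light attenuation and the NSDeactivation effect's Radius parameter to match.
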(event `self.Sphere.OnComponentBeginOverlap`
  (params (OverlappedComponent :type "PrimitiveComponent Object Reference") (OtherActor :type "Actor Object Reference") (OtherComp :type "PrimitiveComponent Object Reference") (OtherBodyIndex :type Integer) (bFromSweep :type Boolean) (SweepResult :type "HitResult Structure (by ref)"))
  (bind _asbp_weapon (cast `/Game/Blueprints/Weapon/BP_Weapon` OtherActor))
  (`/Game/Blueprints/Weapon/BP_Riffle.SetCondition` _asbp_weapon true false))

(event `self.Sphere.OnComponentEndOverlap`
  (params (OverlappedComponent :type "PrimitiveComponent Object Reference") (OtherActor :type "Actor Object Reference") (OtherComp :type "PrimitiveComponent Object Reference") (OtherBodyIndex :type Integer))
  (bind _asbp_weapon (cast `/Game/Blueprints/Weapon/BP_Weapon` OtherActor))
  (`/Game/Blueprints/Weapon/BP_Riffle.SetCondition` _asbp_weapon false false))

(fn `UserConstructionScript`
  (bind (_returnvalue_x _returnvalue_y _returnvalue_z) (`KismetMathLibrary.BreakVector` (`SceneComponent.K2_GetComponentScale` (`self.Sphere`))))
  (bind _returnvalue (* _returnvalue_z 100.0))
  (`LocalLightComponent.SetAttenuationRadius` (`self.PointLight`) _returnvalue)
  (`FXSystemComponent.SetFloatParameter` (`self.NS_Deactivation`) "Radius" _returnvalue))