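; BP_Redirector is an actor that responds to overlapping projectiles by emitting a new BP_Projectile from its own spawn point.
; The new projectile takes the spawn point's location and rotation and the incoming actor's scale; the incoming actor is left untouched here.
; A short time gate throttles overlaps, updating before the Projectile tag check.
; The construction script randomises the mesh material and arrow colour.
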(event `self.ReceiveActorBeginOverlap`
  (params (OtherActor :type "Actor Object Reference"))
  (bind _projectilespawn (`self.ProjectileSpawn`))
  (bind _output_get (set `self.CurrentTime` (`KismetSystemLibrary.GetGameTimeInSeconds`)))
  (if (> (- _output_get (`self.LastCallTime`)) 0.08)
    (set `self.LastCallTime` (`self.CurrentTime`))
    (if (`self.ActorHasTag` OtherActor "Projectile")
      (`|SpawnActorFromClass` "/Game/Blueprints/Weapon/BP_Projectile.BP_Projectile_C" (`KismetMathLibrary.MakeTransform` (`SceneComponent.K2_GetComponentLocation` _projectilespawn) (`SceneComponent.K2_GetComponentRotation` _projectilespawn) (`self.GetActorScale3D` OtherActor)) "Undefined" "OverrideRootScale" null null))))

(fn `UserConstructionScript`
  (`PrimitiveComponent.SetMaterial` (`self.StaticMesh`) 0 (`/Game/Blueprints/Game/BFL_Main.Get Random Material`))
  (`ArrowComponent.SetArrowColor` (`self.Arrow`) (`/Game/Blueprints/Game/BFL_Main.Get Random Emissive Linear Color`)))