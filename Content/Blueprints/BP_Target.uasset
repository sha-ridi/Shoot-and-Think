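; BP_Target is a shootable level objective that turns from red to green when a projectile hits it.
; On BeginPlay it registers with BP_LevelController as an activatable.
; The first overlap of its Cylinder by a "Projectile"-tagged actor sets green solid and emissive materials and asks the controller to end the level if it is the last.
; Every overlapping projectile is destroyed.
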(event `self.ReceiveBeginPlay`
  (`self.SetColor` false)
  (bind _returnvalue (`GameplayStatics.GetActorOfClass` "/Game/Blueprints/BP_LevelController.BP_LevelController_C"))
  (bind _output_get (set `self.Level Controller` _returnvalue))
  (`/Game/Blueprints/BP_LevelController.Add Activatable` _output_get))

(event `self.Cylinder.OnComponentBeginOverlap`
  (params (OverlappedComponent :type "PrimitiveComponent Object Reference") (OtherActor :type "Actor Object Reference") (OtherComp :type "PrimitiveComponent Object Reference") (OtherBodyIndex :type Integer) (bFromSweep :type Boolean) (SweepResult :type "HitResult Structure (by ref)"))
  (if (`self.ActorHasTag` OtherActor "Projectile")
    (`|ExecutionSequence`
      (:`then_0`
        (`/Engine/EditorBlueprintResources/StandardMacros.DoOnce` false
          (:`Completed`
            (`self.SetColor` true)
            (`/Game/Blueprints/BP_LevelController.End Level if Last` (`self.Level Controller`)))))
      (:`then_1`
        (`self.K2_DestroyActor` OtherActor)))))

(fn `SetColor`
  (params (bGreen :type Boolean))
  (`PrimitiveComponent.SetMaterial` (`self.Cylinder`) 0 (select `bool` (`local.bGreen`) :`false` "/Game/Assets/Materials/MI_Red.MI_Red" :`true` "/Game/Assets/Materials/MI_Green.MI_Green" :!type "MaterialInterface Object Reference"))
  (`PrimitiveComponent.SetMaterial` (`self.Cylinder2`) 0 (select `bool` (`local.bGreen`) :`false` "/Game/Assets/Materials/MI_Red.MI_Red" :`true` "/Game/Assets/Materials/MI_Green.MI_Green" :!type "MaterialInterface Object Reference"))
  (`PrimitiveComponent.SetMaterial` (`self.Cylinder3`) 0 (select `bool` (`local.bGreen`) :`false` "/Game/Assets/Materials/MI_EmissiveRed.MI_EmissiveRed" :`true` "/Game/Assets/Materials/MI_EmissiveGreen.MI_EmissiveGreen" :!type "MaterialInterface Object Reference"))
  (`PrimitiveComponent.SetMaterial` (`self.Cylinder1`) 0 (select `bool` (`local.bGreen`) :`false` "/Game/Assets/Materials/MI_EmissiveRed.MI_EmissiveRed" :`true` "/Game/Assets/Materials/MI_EmissiveGreen.MI_EmissiveGreen" :!type "MaterialInterface Object Reference")))

(fn `UserConstructionScript`)