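; Grabbable sphere prop that takes on a random material and gets a toss when released.
; The construction script and BeginPlay each assign a material from GetRandomMaterial, so it is picked again when play begins.
; When GrabComponent fires OnDropped, the sphere receives a mass-dependent impulse scaled up from the actor's current velocity.
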(event `self.ReceiveBeginPlay`
  (`PrimitiveComponent.SetMaterial` (`self.Sphere`) 0 (`/Game/Blueprints/Game/BFL_Main.Get Random Material` false)))

(event `self.GrabComponent.OnDropped`
  (`PrimitiveComponent.AddImpulse` (`self.Sphere`) (* (`self.GetVelocity`) 2.0) "None" false))

(fn `UserConstructionScript`
  (`PrimitiveComponent.SetMaterial` (`self.Sphere`) 0 (`/Game/Blueprints/Game/BFL_Main.Get Random Material` false)))