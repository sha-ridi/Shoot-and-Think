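; BP_Bubble is an environment bubble actor that varies its look and size and drifts off in a random direction.
; The construction script gives the mesh a random material and uniform scale.
; BeginPlay rolls both again, so the placed look is not kept at runtime, then sets a fixed-speed physics velocity along a random unit vector.
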(event `self.ReceiveBeginPlay`
  (`PrimitiveComponent.SetMaterial` (`self.Mesh`) 0 (`/Game/Blueprints/Game/BFL_Main.Get Random Material` true))
  (`SceneComponent.SetWorldScale3D` (`self.Mesh`) (`KismetMathLibrary.Conv_DoubleToVector` (`KismetMathLibrary.RandomFloatInRange` 0.2 0.6)))
  (`PrimitiveComponent.SetPhysicsLinearVelocity` (`self.Mesh`) (* (`KismetMathLibrary.RandomUnitVector`) 70.0) false "None"))

(fn `UserConstructionScript`
  (`SceneComponent.SetWorldScale3D` (`self.Mesh`) (`KismetMathLibrary.Conv_DoubleToVector` (`KismetMathLibrary.RandomFloatInRange` 0.2 0.6)))
  (`PrimitiveComponent.SetMaterial` (`self.Mesh`) 0 (`/Game/Blueprints/Game/BFL_Main.Get Random Material` true)))