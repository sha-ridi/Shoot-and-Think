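; Environment block with a scaled twin mesh that mirrors the original block's movement at a separate location.
; Each Tick, the copy is placed at TwinLocation plus the original's offset from its construction-time start, multiplied by TwinScale, and matches its rotation.
; Construction and BeginPlay assign random materials to both meshes and size the copy by TwinScale.
; Projectiles that overlap the copy are destroyed.
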(event `self.ReceiveBeginPlay`
  (`self.Set Appearance`))

(event `self.ReceiveTick`
  (params (DeltaSeconds :type "Float (single-precision)"))
  (`self.Set Twin Transform` (`self.Start Location`)))

(event `self.SM_Copy.OnComponentBeginOverlap`
  (params (OverlappedComponent :type "PrimitiveComponent Object Reference") (OtherActor :type "Actor Object Reference") (OtherComp :type "PrimitiveComponent Object Reference") (OtherBodyIndex :type Integer) (bFromSweep :type Boolean) (SweepResult :type "HitResult Structure (by ref)"))
  (bind _asbp_projectile (cast `/Game/Blueprints/Weapon/BP_Projectile` OtherActor))
  (`self.K2_DestroyActor` _asbp_projectile))

(fn `Set Appearance`
  (`PrimitiveComponent.SetMaterial` (`self.SM_Origin`) 0 (`/Game/Blueprints/Game/BFL_Main.Get Random Material` false))
  (`PrimitiveComponent.SetMaterial` (`self.SM_Copy`) 0 (`/Game/Blueprints/Game/BFL_Main.Get Random Material` false))
  (`SceneComponent.SetWorldScale3D` (`self.SM_Copy`) (* (`SceneComponent.K2_GetComponentScale` (`self.SM_Origin`)) (`self.Twin Scale`))))

(fn `Set Twin Transform`
  (params (`Start Location` :type "Vector Structure"))
  (`SceneComponent.K2_SetWorldLocation` (`self.SM_Copy`) (+ (`self.TwinLocation`) (* (- (`SceneComponent.K2_GetComponentLocation` (`self.SM_Origin`)) `Start Location`) (`self.Twin Scale`))) false false)
  (`SceneComponent.K2_SetWorldRotation` (`self.SM_Copy`) (`SceneComponent.K2_GetComponentRotation` (`self.SM_Origin`)) false false))

(fn `UserConstructionScript`
  (bind _output_get (set `self.Start Location` (`self.K2_GetActorLocation`)))
  (`self.Set Twin Transform` _output_get)
  (`self.Set Appearance`))