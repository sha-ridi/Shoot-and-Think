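; BP_Block is an environment block with a Cube component that can take on a random look.
; When RandomColor is set, it applies the result of GetRandomMaterial to the cube's first material slot.
; This runs in both the Construction Script and BeginPlay, so the material chosen at construction is picked again when play begins.
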(event `self.ReceiveBeginPlay`
  (if (`self.bRandomColor`)
    (`PrimitiveComponent.SetMaterial` (`self.Cube`) 0 (`/Game/Blueprints/Game/BFL_Main.Get Random Material`))))

(fn `UserConstructionScript`
  (if (`self.bRandomColor`)
    (`PrimitiveComponent.SetMaterial` (`self.Cube`) 0 (`/Game/Blueprints/Game/BFL_Main.Get Random Material`))))