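; BP_VisWall is an environment wall piece that registers a deactivator on any BP_Weapon overlapping its Deactivator component.
; Overlap begin and end call the weapon's AddDeactivator and RemoveDeactivator.
; The construction script pins the world-space thickness of four edge cubes while preserving their lengths from Cube and Cube2.
; Construction and BeginPlay both apply GetRandomMaterial results to those edges and four small cubes.
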(event `self.ReceiveBeginPlay`
  (`PrimitiveComponent.SetMaterial` (`self.Cube1`) 0 (`/Game/Blueprints/Game/BFL_Main.Get Random Material` false))
  (`PrimitiveComponent.SetMaterial` (`self.Cube`) 0 (`/Game/Blueprints/Game/BFL_Main.Get Random Material` false))
  (`PrimitiveComponent.SetMaterial` (`self.Cube2`) 0 (`/Game/Blueprints/Game/BFL_Main.Get Random Material` false))
  (`PrimitiveComponent.SetMaterial` (`self.Cube3`) 0 (`/Game/Blueprints/Game/BFL_Main.Get Random Material` false))
  (`PrimitiveComponent.SetMaterial` (`self.SmallCube`) 0 (`/Game/Blueprints/Game/BFL_Main.Get Random Material` false))
  (`PrimitiveComponent.SetMaterial` (`self.SmallCube1`) 0 (`/Game/Blueprints/Game/BFL_Main.Get Random Material` false))
  (`PrimitiveComponent.SetMaterial` (`self.SmallCube2`) 0 (`/Game/Blueprints/Game/BFL_Main.Get Random Material` false))
  (`PrimitiveComponent.SetMaterial` (`self.SmallCube3`) 0 (`/Game/Blueprints/Game/BFL_Main.Get Random Material` false)))

(event `self.Deactivator.OnComponentBeginOverlap`
  (params (OverlappedComponent :type "PrimitiveComponent Object Reference") (OtherActor :type "Actor Object Reference") (OtherComp :type "PrimitiveComponent Object Reference") (OtherBodyIndex :type Integer) (bFromSweep :type Boolean) (SweepResult :type "HitResult Structure (by ref)"))
  (bind _asbp_weapon (cast `/Game/Blueprints/Weapon/BP_Weapon` OtherActor))
  (`/Game/Blueprints/Weapon/BP_Weapon.Add Deactivator` _asbp_weapon))

(event `self.Deactivator.OnComponentEndOverlap`
  (params (OverlappedComponent :type "PrimitiveComponent Object Reference") (OtherActor :type "Actor Object Reference") (OtherComp :type "PrimitiveComponent Object Reference") (OtherBodyIndex :type Integer))
  (bind _asbp_weapon (cast `/Game/Blueprints/Weapon/BP_Weapon` OtherActor))
  (`/Game/Blueprints/Weapon/BP_Weapon.Remove Deactivator` _asbp_weapon))

(fn `UserConstructionScript`
  (bind _returnvalue_x (`KismetMathLibrary.BreakVector` (`SceneComponent.K2_GetComponentScale` (`self.Cube2`))))
  (bind (_returnvalue_x_2 _returnvalue_y) (`KismetMathLibrary.BreakVector` (`SceneComponent.K2_GetComponentScale` (`self.Cube`))))
  (`SceneComponent.SetWorldScale3D` (`self.Cube`) (`KismetMathLibrary.MakeVector` 0.1 _returnvalue_y 0.1))
  (`SceneComponent.SetWorldScale3D` (`self.Cube1`) (`KismetMathLibrary.MakeVector` 0.1 _returnvalue_y 0.1))
  (`SceneComponent.SetWorldScale3D` (`self.Cube2`) (`KismetMathLibrary.MakeVector` _returnvalue_x 0.1 0.1))
  (`SceneComponent.SetWorldScale3D` (`self.Cube3`) (`KismetMathLibrary.MakeVector` _returnvalue_x 0.1 0.1))
  (`PrimitiveComponent.SetMaterial` (`self.Cube1`) 0 (`/Game/Blueprints/Game/BFL_Main.Get Random Material` false))
  (`PrimitiveComponent.SetMaterial` (`self.Cube`) 0 (`/Game/Blueprints/Game/BFL_Main.Get Random Material` false))
  (`PrimitiveComponent.SetMaterial` (`self.Cube2`) 0 (`/Game/Blueprints/Game/BFL_Main.Get Random Material` false))
  (`PrimitiveComponent.SetMaterial` (`self.Cube3`) 0 (`/Game/Blueprints/Game/BFL_Main.Get Random Material` false))
  (`PrimitiveComponent.SetMaterial` (`self.SmallCube`) 0 (`/Game/Blueprints/Game/BFL_Main.Get Random Material` false))
  (`PrimitiveComponent.SetMaterial` (`self.SmallCube1`) 0 (`/Game/Blueprints/Game/BFL_Main.Get Random Material` false))
  (`PrimitiveComponent.SetMaterial` (`self.SmallCube2`) 0 (`/Game/Blueprints/Game/BFL_Main.Get Random Material` false))
  (`PrimitiveComponent.SetMaterial` (`self.SmallCube3`) 0 (`/Game/Blueprints/Game/BFL_Main.Get Random Material` false)))