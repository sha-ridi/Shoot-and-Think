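; BFL_Main is a Blueprint function library with helpers for random color materials and level progression.
; GetRandomColorMaterial picks among four blue material instances by random index, though its 0 to 4 range exceeds the four options.
; GetNextLevelName strips "Level" from the current level name, increments the number and returns the rebuilt "LevelN" Name, relying on that naming convention.
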(fn `Get Next Level Name`
  (returns (ReturnValue :type Name))
  (bind _returnvalue (`GameplayStatics.GetCurrentLevelName` null))
  (bind _result (`/Engine/EditorBlueprintResources/StandardMacros.IncrementInt` (`KismetStringLibrary.Conv_StringToInt` (`KismetStringLibrary.Replace` _returnvalue "Level")))
    (:`  `
      (return (`KismetStringLibrary.Conv_StringToName` (`KismetStringLibrary.Concat_StrStr` "Level" (`KismetStringLibrary.Conv_IntToString` _result)))))))

(fn `Get Random Color Material`
  (returns (ReturnValue :type "MaterialInterface Object Reference"))
  (return (select `int` (`KismetMathLibrary.RandomIntegerInRange` 0 4) :`0` "/Game/Assets/Materials/MI_DarkBlue.MI_DarkBlue" :`1` "/Game/Assets/Materials/MI_NormalBlue.MI_NormalBlue" :`2` "/Game/Assets/Materials/MI_LightLightBlue.MI_LightLightBlue" :`3` "/Game/Assets/Materials/MI_LightBlue.MI_LightBlue" :!type "MaterialInterface Object Reference")))